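; BP_FlyingCamera is the auto-scrolling camera for the Crossy Road-style game, moving forward along X every tick.
; Each tick it scales BaseSpeed by how far the player chicken is beyond a minimum X distance, never dropping below base speed, so it catches up when the chicken runs ahead.
; WatchHawkGrabChicken stops the scrolling and snaps the camera to that minimum X distance behind the chicken.
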(event `self.ReceiveBeginPlay`
  (bind _asbp_chicken (cast `/Game/CrossyRoad/Blueprints/BP_Chicken` (`GameplayStatics.GetPlayerPawn` 0)))
  (set `self.Chicken` _asbp_chicken))

(event `self.ReceiveTick`
  (params (DeltaSeconds :type "Float (single-precision)"))
  (`self.UpdateCameraSpeed`)
  (`self.K2_SetActorLocation` (+ (`self.K2_GetActorLocation`) (`KismetMathLibrary.MakeVector` (* DeltaSeconds (`self.CurrentSpeed`))))))

(fn `GetXDistanceFromChicken`
  (returns (XDistanceFromChicken :type "Float (double-precision)"))
  (bind _returnvalue_x (`KismetMathLibrary.BreakVector` (- (`self.K2_GetActorLocation` (`self.Chicken`)) (`self.K2_GetActorLocation`))))
  (return _returnvalue_x))

(fn `UpdateCameraSpeed`
  (bind _xdistancefromchicken (`self.GetXDistanceFromChicken`))
  (set `self.CurrentSpeed` (* (`self.BaseSpeed`) (`KismetMathLibrary.FMax` (/ (- _xdistancefromchicken (`self.MinimumXDistanceFromChicken`)) 120.0) 1.0)))
  (return))

(fn `UserConstructionScript`)

(fn `WatchHawkGrabChicken`
  (bind (_returnvalue_x _returnvalue_y _returnvalue_z) (`KismetMathLibrary.BreakVector` (`self.K2_GetActorLocation`)))
  (bind _returnvalue_x_2 (`KismetMathLibrary.BreakVector` (`self.K2_GetActorLocation` (`self.Chicken`))))
  (set `self.BaseSpeed` 0.0)
  (`self.K2_SetActorLocation` (`KismetMathLibrary.MakeVector` (- _returnvalue_x_2 (`self.MinimumXDistanceFromChicken`)) _returnvalue_y _returnvalue_z)))