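; Floor tile for a Crossy Road-style game that randomly dresses itself with rocks, trees or a coin.
; The construction script caches the relative transforms of rock and tree marker components, then always adds one rock child actor at a random rock point.
; A second roll adds a tree, a coin at one of two points, or another rock, which can share the first rock's point.
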(fn `SetRockPoints`
  (set `self.RockPoints` (`|MakeArray` (`SceneComponent.GetRelativeTransform` (`self.RockPointB`)) (`SceneComponent.GetRelativeTransform` (`self.RockPointC`)) (`SceneComponent.GetRelativeTransform` (`self.RockPoint`)))))

(fn `SetTreePoints`
  (set `self.TreePoints` (`|MakeArray` (`SceneComponent.GetRelativeTransform` (`self.SpawnPointL`)) (`SceneComponent.GetRelativeTransform` (`self.SpawnPointR`)) (`SceneComponent.GetRelativeTransform` (`self.SpawnPoint`)) (`SceneComponent.GetRelativeTransform` (`self.TreeVariantC`)) (`SceneComponent.GetRelativeTransform` (`self.TreeVariantB`)))))

(fn `SpawnGrassCoin`
  (switch `int` (`KismetMathLibrary.RandomIntegerInRange` 0 1)
    (:`Default`
      (`AddComponent|NODE_AddChildActorComponent-2` :`RelativeTransform` (`SceneComponent.GetRelativeTransform` (`self.CoinPointB`)) :!label _label))
    (:`0`
      (goto _label))
    (:`1`
      (`AddComponent|NODE_AddChildActorComponent-3` :`RelativeTransform` (`SceneComponent.GetRelativeTransform` (`self.CoinPointC`))))))

(fn `SpawnMoreTree`
  (bind _treepoints (`self.TreePoints`))
  (`AddComponent|NODE_AddChildActorComponent-1` :`RelativeTransform` (`|GetArrayItem` _treepoints (`KismetMathLibrary.RandomIntegerInRange` 0 (`KismetArrayLibrary.Array_LastIndex` _treepoints)))))

(fn `SpawnRock`
  (bind _rockpoints (`self.RockPoints`))
  (`AddComponent|NODE_AddChildActorComponent-0` :`RelativeTransform` (`|GetArrayItem` _rockpoints (`KismetMathLibrary.RandomIntegerInRange` 0 (`KismetArrayLibrary.Array_LastIndex` _rockpoints)))))

(fn `UserConstructionScript`
  (`self.SetRockPoints`)
  (`self.SetTreePoints`)
  (`self.SpawnRock`)
  (switch `int` (`KismetMathLibrary.RandomIntegerInRange` 0 2)
    (:`Default`
      (`self.SpawnMoreTree` :!label _label))
    (:`0`
      (goto _label))
    (:`1`
      (`self.SpawnGrassCoin`))
    (:`2`
      (`self.SpawnRock`))))