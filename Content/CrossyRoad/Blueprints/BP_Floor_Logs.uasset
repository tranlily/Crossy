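; River floor Blueprint in a Crossy Road-style game that spawns logs and drowns chickens touching the water.
; SpawnLog adds a child actor component at LogPoint's relative transform, once in the construction script and then repeatedly at random intervals of a few seconds.
; The repeat timing comes from a Delay on Tick rather than a timer.
; An overlap with the Box calls Drown on any BP_Chicken that is not already dead.
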(event `self.ReceiveTick`
  (params (DeltaSeconds :type "Float (single-precision)"))
  ;[1 1 1] Every 3-6 seconds, spawn a Log in the river
  (`KismetSystemLibrary.Delay` (`KismetMathLibrary.Conv_IntToDouble` (`KismetMathLibrary.RandomIntegerInRange` 3 6)))
  (`self.SpawnLog`))

(event `self.Box.OnComponentBeginOverlap`
  (params (OverlappedComponent :type "PrimitiveComponent Object Reference") (OtherActor :type "Actor Object Reference") (OtherComp :type "PrimitiveComponent Object Reference") (OtherBodyIndex :type Integer) (bFromSweep :type Boolean) (SweepResult :type "HitResult Structure (by ref)"))
  (bind _asbp_chicken (cast `/Game/CrossyRoad/Blueprints/BP_Chicken` OtherActor))
  (if (not (`/Game/CrossyRoad/Blueprints/BP_Chicken.IsDead` _asbp_chicken))
    (`/Game/CrossyRoad/Blueprints/BP_Chicken.Drown` _asbp_chicken)))

(fn `SpawnLog`
  (`AddComponent|NODE_AddChildActorComponent-0` :`RelativeTransform` (`SceneComponent.GetRelativeTransform` (`self.LogPoint`))))

(fn `UserConstructionScript`
  (`self.SpawnLog`))