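; BP_CrossyLog is a moving log actor in a Crossy Road-style game that reacts to BP_Chicken.
; Tick offsets it along world Y by Speed scaled by delta time, without sweeping.
; A Box overlap with the chicken plays a creak sound, using a flag and a delay matching the clip length to prevent overlapping playback.
; It destroys itself when its InterpToMovement component stops.
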(event `self.ReceiveTick`
  (params (DeltaSeconds :type "Float (single-precision)"))
  (`self.K2_SetActorLocation` (+ (`self.K2_GetActorLocation`) (`KismetMathLibrary.MakeVector` 0.0 (* DeltaSeconds (`self.Speed`))))))

(event `self.Box.OnComponentBeginOverlap`
  (params (OverlappedComponent :type "PrimitiveComponent Object Reference") (OtherActor :type "Actor Object Reference") (OtherComp :type "PrimitiveComponent Object Reference") (OtherBodyIndex :type Integer) (bFromSweep :type Boolean) (SweepResult :type "HitResult Structure (by ref)"))
  (cast `/Game/CrossyRoad/Blueprints/BP_Chicken` OtherActor)
  (if (not (`self.IsSoundPlaying`))
    (`GameplayStatics.PlaySoundAtLocation` "/Game/CrossyRoad/CrossyAudio/logcreak.logcreak" (`self.K2_GetActorLocation`) (struct) 1.0 1.0 0.0 null null null)
    (set `self.IsSoundPlaying` true)
    (`KismetSystemLibrary.Delay` 0.5) ; 0.5 seconds is the length of the sound file.
    (set `self.IsSoundPlaying` false)))

(event `self.InterpToMovement.OnInterpToStop`
  (params (ImpactResult :type "HitResult Structure (by ref)") (Time :type "Float (single-precision)"))
  (`self.K2_DestroyActor`))

(fn `UserConstructionScript`)