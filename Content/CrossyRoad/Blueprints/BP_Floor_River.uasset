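; BP_Floor_River is a river floor piece for a Crossy Road-style game that drowns a living BP_Chicken when it overlaps the Box.
; The construction script gathers four pad transforms and spawns a lilypad child actor at a random one.
; It then randomly adds either another lilypad, which may land on the same point, or two child actors at the fixed coin pad and coin points.
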(event `self.Box.OnComponentBeginOverlap`
  (params (OverlappedComponent :type "PrimitiveComponent Object Reference") (OtherActor :type "Actor Object Reference") (OtherComp :type "PrimitiveComponent Object Reference") (OtherBodyIndex :type Integer) (bFromSweep :type Boolean) (SweepResult :type "HitResult Structure (by ref)"))
  (bind _asbp_chicken (cast `/Game/CrossyRoad/Blueprints/BP_Chicken` OtherActor))
  (if (not (`/Game/CrossyRoad/Blueprints/BP_Chicken.IsDead` _asbp_chicken))
    (`/Game/CrossyRoad/Blueprints/BP_Chicken.Drown` _asbp_chicken)))

(fn `SetLilypadPoints`
  (set `self.LilypadPoints` (`|MakeArray` (`SceneComponent.GetRelativeTransform` (`self.PadPointA`)) (`SceneComponent.GetRelativeTransform` (`self.PadPointB`)) (`SceneComponent.GetRelativeTransform` (`self.PadPoint`)) (`SceneComponent.GetRelativeTransform` (`self.PadPointC`)))))

(fn `SpawnCoin`
  (`AddComponent|NODE_AddChildActorComponent-4` :`RelativeTransform` (`SceneComponent.GetRelativeTransform` (`self.CoinPadA`)))
  (`AddComponent|NODE_AddChildActorComponent-5` :`RelativeTransform` (`SceneComponent.GetRelativeTransform` (`self.CoinPointA`))))

(fn `SpawnLilypad`
  (bind _lilypadpoints (`self.LilypadPoints`))
  (`AddComponent|NODE_AddChildActorComponent-0` :`RelativeTransform` (`|GetArrayItem` _lilypadpoints (`KismetMathLibrary.RandomIntegerInRange` 0 (`KismetArrayLibrary.Array_LastIndex` _lilypadpoints)))))

(fn `UserConstructionScript`
  (`self.SetLilypadPoints`)
  (`self.SpawnLilypad`)
  (switch `int` (`KismetMathLibrary.RandomIntegerInRange` 0 1)
    (:`Default`
      (`self.SpawnLilypad` :!label _label))
    (:`0`
      (goto _label))
    (:`1`
      (`self.SpawnCoin`))))