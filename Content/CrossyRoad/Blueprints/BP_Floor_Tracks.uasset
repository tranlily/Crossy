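; BP_Floor_Tracks is a Crossy Road railway floor piece that lays tracks, places a light post and periodically spawns trains.
; The construction script gathers marker component transforms into TrackPoints, then adds child actor components for each track segment and the light post.
; Tick uses a random 6–8 second Delay as a repeating timer, adding a train child actor at TrainPoint, then playing a bell sound at world origin.
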(event `self.ReceiveTick`
  (params (DeltaSeconds :type "Float (single-precision)"))
  ;[1 1 1] Every 6-8 seconds, spawn a Train
  (`KismetSystemLibrary.Delay` (`KismetMathLibrary.Conv_IntToDouble` (`KismetMathLibrary.RandomIntegerInRange` 6 8)))
  (`self.SpawnTrain`)
  (`GameplayStatics.PlaySoundAtLocation` "/Game/CrossyRoad/CrossyAudio/bell.bell" (0.0 0.0 0.0) (struct) 1.0 1.0 0.0 null null null))

(fn `SetTrackPoints`
  (set `self.TrackPoints` (`|MakeArray` (`SceneComponent.GetRelativeTransform` (`self.TrackPoint`)) (`SceneComponent.GetRelativeTransform` (`self.TrackPointA`)) (`SceneComponent.GetRelativeTransform` (`self.TrackPointB`)) (`SceneComponent.GetRelativeTransform` (`self.TrackPointC`)) (`SceneComponent.GetRelativeTransform` (`self.TrackPointD`)) (`SceneComponent.GetRelativeTransform` (`self.TrackPointE`)) (`SceneComponent.GetRelativeTransform` (`self.TrackPointF`)) (`SceneComponent.GetRelativeTransform` (`self.TrackPointG`)) (`SceneComponent.GetRelativeTransform` (`self.TrackPointH`)) (`SceneComponent.GetRelativeTransform` (`self.TrackPointI`)) (`SceneComponent.GetRelativeTransform` (`self.TrackPointJ`)) (`SceneComponent.GetRelativeTransform` (`self.TrackPointK`)) (struct) (struct))))

(fn `SpawnLightpost`
  (`AddComponent|NODE_AddChildActorComponent-15` :`RelativeTransform` (`SceneComponent.GetRelativeTransform` (`self.LightPoint`))))

(fn `SpawnTracks`
  (`AddComponent|NODE_AddChildActorComponent-0` :`RelativeTransform` (`|GetArrayItem` (`self.TrackPoints`)))
  (`AddComponent|NODE_AddChildActorComponent-2` :`RelativeTransform` (`|GetArrayItem` (`self.TrackPoints`) 1))
  (`AddComponent|NODE_AddChildActorComponent-3` :`RelativeTransform` (`|GetArrayItem` (`self.TrackPoints`) 2))
  (`AddComponent|NODE_AddChildActorComponent-4` :`RelativeTransform` (`|GetArrayItem` (`self.TrackPoints`) 3))
  (`AddComponent|NODE_AddChildActorComponent-5` :`RelativeTransform` (`|GetArrayItem` (`self.TrackPoints`) 4))
  (`AddComponent|NODE_AddChildActorComponent-6` :`RelativeTransform` (`|GetArrayItem` (`self.TrackPoints`) 5))
  (`AddComponent|NODE_AddChildActorComponent-7` :`RelativeTransform` (`|GetArrayItem` (`self.TrackPoints`) 6))
  (`AddComponent|NODE_AddChildActorComponent-8` :`RelativeTransform` (`|GetArrayItem` (`self.TrackPoints`) 7))
  (`AddComponent|NODE_AddChildActorComponent-9` :`RelativeTransform` (`|GetArrayItem` (`self.TrackPoints`) 8))
  (`AddComponent|NODE_AddChildActorComponent-10` :`RelativeTransform` (`|GetArrayItem` (`self.TrackPoints`) 9))
  (`AddComponent|NODE_AddChildActorComponent-16` :`RelativeTransform` (`|GetArrayItem` (`self.TrackPoints`) 10))
  (`AddComponent|NODE_AddChildActorComponent-17` :`RelativeTransform` (`|GetArrayItem` (`self.TrackPoints`) 11)))

(fn `SpawnTrain`
  (`AddComponent|NODE_AddChildActorComponent-1` :`RelativeTransform` (`SceneComponent.GetRelativeTransform` (`self.TrainPoint`))))

(fn `UserConstructionScript`
  (`self.SetTrackPoints`)
  (`self.SpawnTracks`)
  (`self.SpawnLightpost`))