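; BP_Floor is an endless-runner floor tile for the Crossy Road game that chains new tiles as the chicken advances.
; Construction gathers three spawn points, then adds a child actor at a random one and others at two tree points.
; When BP_Chicken first overlaps EndTrigger, it scores, RunGameMode adds a tile, and this one destroys itself after a delay.
; GetAttachTransform exposes the AttachPoint world transform.
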(event `self.EndTrigger.OnComponentBeginOverlap`
  (params (OverlappedComponent :type "PrimitiveComponent Object Reference") (OtherActor :type "Actor Object Reference") (OtherComp :type "PrimitiveComponent Object Reference") (OtherBodyIndex :type Integer) (bFromSweep :type Boolean) (SweepResult :type "HitResult Structure (by ref)"))
  (bind _asbp_chicken (cast `/Game/CrossyRoad/Blueprints/BP_Chicken` OtherActor))
  (bind _asrun_game_mode (cast `/Game/CrossyRoad/Blueprints/RunGameMode` (`GameplayStatics.GetGameMode`)))
  (if (not (`self.HasGivenPoints`))
    (set `self.HasGivenPoints` true)
    (`/Engine/EditorBlueprintResources/StandardMacros.IncrementInt` (`/Game/CrossyRoad/Blueprints/BP_Chicken.Score` _asbp_chicken)
      (:`  `
        (`/Game/CrossyRoad/Blueprints/RunGameMode.AddFloorTile` _asrun_game_mode)
        (`KismetSystemLibrary.Delay` 9.0)
        (`self.K2_DestroyActor`)))))

(fn `GetAttachTransform`
  (returns (AttachTransform :type "Transform Structure"))
  (return (`SceneComponent.K2_GetComponentToWorld` (`self.AttachPoint`))))

(fn `SetSpawnPoints`
  (set `self.SpawnPoints` (`|MakeArray` (`SceneComponent.GetRelativeTransform` (`self.SpawnPoint`)) (`SceneComponent.GetRelativeTransform` (`self.SpawnPointL`)) (`SceneComponent.GetRelativeTransform` (`self.SpawnPointR`)))))

(fn `SpawnTree`
  (bind _spawnpoints (`self.SpawnPoints`))
  (bind _returnvalue (`SceneComponent.GetRelativeTransform` (`self.TreePointA`)))
  (bind _returnvalue_2 (`SceneComponent.GetRelativeTransform` (`self.TreePointB`)))
  (`AddComponent|NODE_AddChildActorComponent-0` :`RelativeTransform` (`|GetArrayItem` _spawnpoints (`KismetMathLibrary.RandomIntegerInRange` 0 (`KismetArrayLibrary.Array_LastIndex` _spawnpoints))))
  (switch `int` (`KismetMathLibrary.RandomIntegerInRange` 0 1)
    (:`Default`
      (`AddComponent|NODE_AddChildActorComponent-6` :`RelativeTransform` _returnvalue :!label _label)
      (`AddComponent|NODE_AddChildActorComponent-9` :`RelativeTransform` _returnvalue_2))
    (:`0`
      (`AddComponent|NODE_AddChildActorComponent-7` :`RelativeTransform` _returnvalue)
      (`AddComponent|NODE_AddChildActorComponent-8` :`RelativeTransform` _returnvalue_2))
    (:`1`
      (goto _label))))

(fn `UserConstructionScript`
  (`self.SetSpawnPoints`)
  (switch `int` 0
    (:`Default`
      (`self.SpawnTree`))))