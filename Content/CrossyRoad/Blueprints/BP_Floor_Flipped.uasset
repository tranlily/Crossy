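; BP_Floor_Flipped is a Crossy Road floor piece that keeps spawning red or yellow cars.
; Tick runs into a random two-to-four-second Delay, which paces spawning, then a random switch calls SpawnRedCar or SpawnYellowCar.
; Both functions add a child actor component at CarPointA's relative transform.
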(event `self.ReceiveTick`
  (params (DeltaSeconds :type "Float (single-precision)"))
  (`KismetSystemLibrary.Delay` (`KismetMathLibrary.Conv_IntToDouble` (`KismetMathLibrary.RandomIntegerInRange` 2 4)))
  (switch `int` (`KismetMathLibrary.RandomIntegerInRange` 0 1)
    (:`Default`
      (`self.SpawnRedCar` :!label _label))
    (:`0`
      (goto _label))
    (:`1`
      (`self.SpawnYellowCar`))))

(fn `SpawnRedCar`
  (`AddComponent|NODE_AddChildActorComponent-0` :`RelativeTransform` (`SceneComponent.GetRelativeTransform` (`self.CarPointA`))))

(fn `SpawnYellowCar`
  (`AddComponent|NODE_AddChildActorComponent-1` :`RelativeTransform` (`SceneComponent.GetRelativeTransform` (`self.CarPointA`))))

(fn `UserConstructionScript`
  (`parent.UserConstructionScript`))