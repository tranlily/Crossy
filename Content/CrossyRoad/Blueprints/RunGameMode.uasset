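; Game mode for a Crossy Road-style runner that builds the floor path and manages cameras for BP_Chicken.
; BeginPlay shows a splash while movement is locked, lays safe floors, then adds random floors, HUD and cameras.
; Floors chain through each tile's attach transform, with separate pools for harder levels and highways, not called here.
; Camera functions switch between a flying view and a first-person view with ominous music.
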(event `self.ReceiveBeginPlay`
  (bind _asbp_chicken (cast `/Game/CrossyRoad/Blueprints/BP_Chicken` (`GameplayStatics.GetPlayerPawn` 0)))
  (set `self.Player` _asbp_chicken)
  (`self.PlaySplashScreen`)
  (`self.AddBeginningFloor`)
  (`KismetSystemLibrary.Delay` 2.5) ; Allow intro screen to play out.
  (`/Game/CrossyRoad/Blueprints/BP_Chicken.AllowMovement` (`self.Player`))
  (`self.InitializeFirstLevel`))

(fn `ActivateDefaultCamera`
  (bind _flyingcamera (`self.FlyingCamera`))
  (bind _player (`self.Player`))
  (bind _returnvalue_x (`KismetMathLibrary.BreakVector` (`self.K2_GetActorLocation` (`self.Player`))))
  (bind (_returnvalue_x_2 _returnvalue_y _returnvalue_z) (`KismetMathLibrary.BreakVector` (`self.K2_GetActorLocation` _flyingcamera)))
  (set `/Game/CrossyRoad/Blueprints/BP_Chicken.MainCamera` (`self.FlyingCamera`) _player)
  (set `/Game/CrossyRoad/Blueprints/BP_Chicken.IsFirstPersonModeActive` false _player)
  (`self.K2_SetActorLocation` _flyingcamera (`KismetMathLibrary.MakeVector` (- _returnvalue_x (`/Game/CrossyRoad/Blueprints/BP_FlyingCamera.MinimumXDistanceFromChicken` _flyingcamera)) _returnvalue_y _returnvalue_z) false false)
  (`self.StopOminousMusic`)
  (`PlayerController.SetViewTargetWithBlend` (`GameplayStatics.GetPlayerController` 0) _flyingcamera 0.0 "VTBlend_Linear" 0.0 false))

(fn `ActivateFirstPersonCamera`
  (`self.StartOminousMusic`)
  (set `/Game/CrossyRoad/Blueprints/BP_Chicken.IsFirstPersonModeActive` true (`self.Player`))
  (`PlayerController.SetViewTargetWithBlend` (`GameplayStatics.GetPlayerController` 0) (`self.FirstPersonCamera`) 1.0 "VTBlend_Linear" 0.0 false))

(fn `AddBeginningFloor`
  (bind _safetiles (`self.SafeTiles`))
  (for _ (range 3)
    (bind _returnvalue (`|SpawnActorFromClass` (`|GetArrayItem` _safetiles (`KismetMathLibrary.RandomIntegerInRange` 0 (`KismetArrayLibrary.Array_LastIndex` _safetiles))) (`self.NextSpawnPoint`) "Undefined" "OverrideRootScale" null null))
    (bind _asbp_floor (cast `/Game/CrossyRoad/Blueprints/BP_Floor` _returnvalue))
    (bind _attachtransform (`/Game/CrossyRoad/Blueprints/BP_Floor.GetAttachTransform` _asbp_floor))
    (set `self.NextSpawnPoint` _attachtransform)))

(fn `AddFloorTile`
  (bind _floortiles (`self.FloorTiles`))
  ;[1 1 1] Spawns floors completely randomly
  (bind _returnvalue (`|SpawnActorFromClass` (`|GetArrayItem` _floortiles (`KismetMathLibrary.RandomIntegerInRange` 0 (`KismetArrayLibrary.Array_LastIndex` _floortiles))) (`self.NextSpawnPoint`) "Undefined" "OverrideRootScale" null null))
  (bind _asbp_floor (cast `/Game/CrossyRoad/Blueprints/BP_Floor` _returnvalue))
  (bind _attachtransform (`/Game/CrossyRoad/Blueprints/BP_Floor.GetAttachTransform` _asbp_floor))
  (set `self.NextSpawnPoint` _attachtransform))

(fn `CreateOminousMusic`
  (bind _returnvalue (`GameplayStatics.SpawnSound2D` "/Game/CrossyRoad/CrossyAudio/crossysong_Cue.crossysong_Cue" 1.0 1.0 0.0 null))
  (set `self.OminousComponent` _returnvalue))

(fn `IncreaseDifficulty`
  (bind _level2 (`self.Level2`))
  ;[1 1 1] After N Floors, the player gets 1 less safe floor pulled randomly, thus more challenging floors are spawned
  (bind _returnvalue (`|SpawnActorFromClass` (`|GetArrayItem` _level2 (`KismetMathLibrary.RandomIntegerInRange` 0 (`KismetArrayLibrary.Array_LastIndex` _level2))) (`self.NextSpawnPoint`) "Undefined" "OverrideRootScale" null null))
  (bind _asbp_floor (cast `/Game/CrossyRoad/Blueprints/BP_Floor` _returnvalue))
  (bind _attachtransform (`/Game/CrossyRoad/Blueprints/BP_Floor.GetAttachTransform` _asbp_floor))
  (set `self.NextSpawnPoint` _attachtransform))

(fn `InitializeCameras`
  (bind _asbp_chicken (cast `/Game/CrossyRoad/Blueprints/BP_Chicken` (`GameplayStatics.GetPlayerPawn` 0)))
  (bind _returnvalue (`|SpawnActorFromClass` "/Game/CrossyRoad/Blueprints/BP_FlyingCamera.BP_FlyingCamera_C" (`SceneComponent.K2_GetComponentToWorld` (`/Game/CrossyRoad/Blueprints/BP_Chicken.FollowCamera` _asbp_chicken)) "Undefined" "OverrideRootScale" null null))
  (set `self.FlyingCamera` _returnvalue)
  (bind _returnvalue_2 (`|SpawnActorFromClass` "/Game/CrossyRoad/Blueprints/BP_FirstPersonCamera.BP_FirstPersonCamera_C" (`KismetMathLibrary.MakeTransform` (0.0 0.0 0.0)) "Undefined" "OverrideRootScale" null null))
  (set `self.FirstPersonCamera` _returnvalue_2)
  (`self.ActivateDefaultCamera`))

(fn `InitializeFirstLevel`
  ;[1 1 1] Initialize the HUD, Spawn Randomly N floors fairly, amongst all kinds of floors
  (for _ (range 5)
    (`self.AddFloorTile`)
    (bind _returnvalue (`|CreateWidget` "/Game/CrossyRoad/UMG/CrossyHUD.CrossyHUD_C"))
    (`UserWidget.AddToViewport` _returnvalue 0))
  (`self.InitializeCameras`))

(fn `PlaySplashScreen`
  (`/Game/CrossyRoad/Blueprints/BP_Chicken.ForbidMovement` (`self.Player`))
  (bind _returnvalue (`|CreateWidget` "/Game/CrossyRoad/UMG/SplashScreen.SplashScreen_C"))
  (`UserWidget.AddToViewport` _returnvalue 0))

(fn `PullHighways`
  (bind _highways (`self.Highways`))
  ;[1 1 1] The Ceiling difficulty of the game, the purpose is to make it simple to test, by making the game more difficult after N floors
  (bind _returnvalue (`|SpawnActorFromClass` (`|GetArrayItem` _highways (`KismetMathLibrary.RandomIntegerInRange` 0 (`KismetArrayLibrary.Array_LastIndex` _highways))) (`self.NextSpawnPoint`) "Undefined" "OverrideRootScale" null null))
  (bind _asbp_floor (cast `/Game/CrossyRoad/Blueprints/BP_Floor` _returnvalue))
  (bind _attachtransform (`/Game/CrossyRoad/Blueprints/BP_Floor.GetAttachTransform` _asbp_floor))
  (set `self.NextSpawnPoint` _attachtransform))

(fn `StartOminousMusic`
  (bind _ominouscomponent (`self.OminousComponent`))
  (`/Engine/EditorBlueprintResources/StandardMacros.IsValid` _ominouscomponent
    (:`Is Valid`
      _)
    (:`Is Not Valid`
      (`self.CreateOminousMusic`)))
  (`AudioComponent.Play` _ominouscomponent 0.0))

(fn `StopOminousMusic`
  (bind _ominouscomponent (`self.OminousComponent`))
  (`/Engine/EditorBlueprintResources/StandardMacros.IsValid` _ominouscomponent
    (:`Is Valid`
      (`AudioComponent.Stop` _ominouscomponent))))

(fn `UserConstructionScript`)