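; BP_Floor_Road is a road lane floor piece for a Crossy Road style game that spawns traffic.
; Its construction script gathers twelve point transforms and adds a road child actor at each.
; Tick uses a random Delay as a repeating timer to add a car, orange car or truck child actor at its spawn point.
; After each spawn, a coin flip decides whether a delayed horn sound plays at the world origin.
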(event `self.ReceiveTick`
  (params (DeltaSeconds :type "Float (single-precision)"))
  ;[1 1 1] Get the event tick. Between 2-4 seconds, spawn either a Car or a Truck randomly, Randomly choose if a vehicle honks it's horn or doesn't
  (`KismetSystemLibrary.Delay` (`KismetMathLibrary.Conv_IntToDouble` (`KismetMathLibrary.RandomIntegerInRange` 2 4)))
  (switch `int` (`KismetMathLibrary.RandomIntegerInRange` 0 2)
    (:`Default`
      (`self.SpawnCar` :!label _label))
    (:`0`
      (goto _label))
    (:`1`
      (`self.SpawnTruck`))
    (:`2`
      (`self.SpawnOrangeCar`)))
  (switch `int` (`KismetMathLibrary.RandomIntegerInRange` 0 1)
    (:`0`
      (`KismetSystemLibrary.Delay` 2.0))
    (:`1`
      (`KismetSystemLibrary.Delay` (`KismetMathLibrary.Conv_IntToDouble` (`KismetMathLibrary.RandomIntegerInRange` 2 5)))
      (`GameplayStatics.PlaySoundAtLocation` "/Game/CrossyRoad/CrossyAudio/carscreamin.carscreamin" (0.0 0.0 0.0) (struct) 1.0 1.0 0.0 null null null))))

(fn `SetRoadPoints`
  (set `self.Road Points` (`|MakeArray` (`SceneComponent.GetRelativeTransform` (`self.RoadPointA`)) (`SceneComponent.GetRelativeTransform` (`self.RoadPoint`)) (`SceneComponent.GetRelativeTransform` (`self.RoadPointB`)) (`SceneComponent.GetRelativeTransform` (`self.RoadPointC`)) (`SceneComponent.GetRelativeTransform` (`self.RoadPointD`)) (`SceneComponent.GetRelativeTransform` (`self.RoadPointE`)) (`SceneComponent.GetRelativeTransform` (`self.RoadPointF`)) (`SceneComponent.GetRelativeTransform` (`self.RoadPointG`)) (`SceneComponent.GetRelativeTransform` (`self.RoadPointI`)) (`SceneComponent.GetRelativeTransform` (`self.RoadPointJ`)) (`SceneComponent.GetRelativeTransform` (`self.RoadPointH`)) (`SceneComponent.GetRelativeTransform` (`self.RoadPointK`)))))

(fn `SpawnCar`
  (`AddComponent|NODE_AddChildActorComponent-2` :`RelativeTransform` (`SceneComponent.GetRelativeTransform` (`self.CarPoint`))))

(fn `SpawnOrangeCar`
  (`AddComponent|NODE_AddChildActorComponent-11` :`RelativeTransform` (`SceneComponent.GetRelativeTransform` (`self.CarPoint`))))

(fn `SpawnRoad`
  (`AddComponent|NODE_AddChildActorComponent-3` :`RelativeTransform` (`|GetArrayItem` (`self.Road Points`)))
  (`AddComponent|NODE_AddChildActorComponent-4` :`RelativeTransform` (`|GetArrayItem` (`self.Road Points`) 1))
  (`AddComponent|NODE_AddChildActorComponent-5` :`RelativeTransform` (`|GetArrayItem` (`self.Road Points`) 2))
  (`AddComponent|NODE_AddChildActorComponent-6` :`RelativeTransform` (`|GetArrayItem` (`self.Road Points`) 3))
  (`AddComponent|NODE_AddChildActorComponent-7` :`RelativeTransform` (`|GetArrayItem` (`self.Road Points`) 4))
  (`AddComponent|NODE_AddChildActorComponent-8` :`RelativeTransform` (`|GetArrayItem` (`self.Road Points`) 5))
  (`AddComponent|NODE_AddChildActorComponent-9` :`RelativeTransform` (`|GetArrayItem` (`self.Road Points`) 6))
  (`AddComponent|NODE_AddChildActorComponent-10` :`RelativeTransform` (`|GetArrayItem` (`self.Road Points`) 7))
  (`AddComponent|NODE_AddChildActorComponent-12` :`RelativeTransform` (`|GetArrayItem` (`self.Road Points`) 8))
  (`AddComponent|NODE_AddChildActorComponent-13` :`RelativeTransform` (`|GetArrayItem` (`self.Road Points`) 9))
  (`AddComponent|NODE_AddChildActorComponent-14` :`RelativeTransform` (`|GetArrayItem` (`self.Road Points`) 10))
  (`AddComponent|NODE_AddChildActorComponent-15` :`RelativeTransform` (`|GetArrayItem` (`self.Road Points`) 11)))

(fn `SpawnTruck`
  (`AddComponent|NODE_AddChildActorComponent-1` :`RelativeTransform` (`SceneComponent.GetRelativeTransform` (`self.TruckPoint`))))

(fn `UserConstructionScript`
  (`self.SetRoadPoints`)
  (`self.SpawnRoad`))