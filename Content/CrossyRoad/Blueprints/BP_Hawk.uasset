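; BP_Hawk is the hawk that swoops down on the player's chicken and carries it away in a Crossy Road game.
; MoveToChicken caches the chicken's location, plays a scream and runs SwoopTimeline to move the hawk along offsets from that point.
; A timeline event flags the grab, after which the chicken follows at a held offset.
; The swoop assumes the chicken is already locked in place.
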(event `MoveToChicken`
  (bind _asbp_chicken (cast `/Game/CrossyRoad/Blueprints/BP_Chicken` (`GameplayStatics.GetPlayerPawn` 0)))
  (set `self.ChickenInitialPosition` (`self.K2_GetActorLocation` _asbp_chicken))
  (`GameplayStatics.PlaySoundAtLocation` "/Game/CrossyRoad/CrossyAudio/hawkscreamin.hawkscreamin" (`self.K2_GetActorLocation`) (struct) 1.0 1.0 0.0 null null null)
  (bind (_direction _offsetfromplayer) (`Timeline|SwoopTimeline`)
    (:`Update`
      (bind _returnvalue (+ _offsetfromplayer (`self.ChickenInitialPosition`)))
      (`self.K2_SetActorLocation` _returnvalue)
      (if (`self.IsHoldingChicken`)
        (`self.K2_SetActorLocation` _asbp_chicken (+ _returnvalue (`self.HeldChickenOffset`)) false false)))
    (:`ChickenMoveWithHawk`
      (set `self.IsHoldingChicken` true))))

(fn `UserConstructionScript`)